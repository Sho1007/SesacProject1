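; BP_Bullet is a projectile actor that flies along its forward vector and damages actors it overlaps.
; Each Tick calls a Translate helper, which moves the actor by normalized direction × Speed × delta time, with sweep off.
; ActorBeginOverlap applies Damage to the other actor; the bullet is not destroyed on hit.
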(event EventBeginPlay)

(event EventTick
  (params (DeltaSeconds :type Float%20%28single-precision%29))
  ;[1 1 1] 나의 앞 방향으로 이동하고싶다. P=P0+vt
  (CallFunction|Translate (Transformation|GetActorForwardVector) (Variables|Default|GetSpeed) false))

(event Collision|EventActorBeginOverlap
  (params (OtherActor :type Actor%20Object%20Reference))
  (Game|Damage|ApplyDamage OtherActor (Variables|Default|Get%20Damage) 0 0))

(fn ConstructionScript)

(fn Translate
  (params (Direction :type Vector) (Speed :type Float%20%28double-precision%29) (is%20Sweep :type Boolean))
  ;[1 1 1] 속도(Velocity)시간 => vt
  (Transformation|SetActorLocation (+ (Transformation|GetActorLocation) (* (Math|Vector|Normalize Direction) Speed (Utilities|Time|GetWorldDeltaSeconds))) is%20Sweep false))
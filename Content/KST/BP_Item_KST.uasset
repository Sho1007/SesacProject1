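; BP_Item_KST is an experience pickup that homes in on the player and grants EXP on contact.
; BeginPlay caches the first BP_player_KST as the target; any Box overlap permanently switches on homing.
; Tick then moves the item straight toward the target at Speed, scaled by delta time, without sweep.
; A Sphere overlap with a PlayerBase adds a fixed EXP amount and destroys the item.
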(event OnComponentBeginOverlap(Sphere)
  (params (OverlappedComponent :type Primitive%20Component%20Object%20Reference) (OtherActor :type Actor%20Object%20Reference) (OtherComp :type Primitive%20Component%20Object%20Reference) (OtherBodyIndex :type Integer) (bFromSweep :type Boolean) (SweepResult :type Hit%20Result%20Structure%20%28by%20ref%29))
  (bind _asplayer_base (Utilities|Casting|CastToPlayerBase OtherActor))
  (Class|PlayerBase|AddExp _asplayer_base 1e+01)
  (Actor|DestroyActor))

(event OnComponentBeginOverlap(Box)
  (params (OverlappedComponent :type Primitive%20Component%20Object%20Reference) (OtherActor :type Actor%20Object%20Reference) (OtherComp :type Primitive%20Component%20Object%20Reference) (OtherBodyIndex :type Integer) (bFromSweep :type Boolean) (SweepResult :type Hit%20Result%20Structure%20%28by%20ref%29))
  ;[1 1 1] 충돌시 삭제
  (Variables|Default|SetSwich true))

(event EventBeginPlay
  ;[1 1 1] 태어날 때 목적지를 알고싶다
  (bind _returnvalue (Actor|GetActorOfClass "/Game/KST/BP_player_KST.BP_player_KST_C"))
  (Variables|Default|Settarget _returnvalue))

(event Collision|EventActorBeginOverlap
  (params (OtherActor :type Actor%20Object%20Reference)))

(event EventTick
  (params (DeltaSeconds :type Float%20%28single-precision%29))
  (if (Variables|Default|GetSwich)
    (Transformation|SetActorLocation (+ (Transformation|GetActorLocation) (* (Variables|Default|GetSpeed) (Math|Vector|Normalize (- (Transformation|GetActorLocation (Variables|Default|Gettarget)) (Transformation|GetActorLocation))) (Utilities|Time|GetWorldDeltaSeconds))) false false)))

(fn ConstructionScript)
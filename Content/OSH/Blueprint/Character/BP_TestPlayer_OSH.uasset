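; BP_TestPlayer_OSH is a test player that moves on input and fires projectiles automatically.
; BeginPlay adds the default Enhanced Input mapping context, and the move action feeds a normalized direction built from actor right and forward vectors into AddMovementInput, scaled by Speed.
; Tick accumulates time against FireCool and spawns BP_ProjectileBase at Arrow1's transform, carrying leftover time into the next cycle.
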(event Input|EnhancedActionEvents|EnhancedInputActionIA_Move_OSH
  (params (ActionValue :type Vector%202D%20Structure) (ElapsedSeconds :type Float%20%28double-precision%29) (TriggeredSeconds :type Float%20%28double-precision%29) (InputAction :type Input%20Action%20Object%20Reference :default "/Game/OSH/Input/InputAction/IA_Move_OSH.IA_Move_OSH"))
  (bind (_x _y) (Math|Vector2D|BreakVector2D ActionValue))
  (:Triggered
    (Pawn|Input|AddMovementInput (Math|Vector|Normalize (+ (* _x (Transformation|GetActorRightVector)) (* _y (Transformation|GetActorForwardVector)))) (Variables|Default|GetSpeed) false)))

(event EventBeginPlay
  (bind _asplayer_controller (Utilities|Casting|CastToPlayerController (Pawn|GetController)))
  (Input|AddMappingContext (PlayerController|LocalPlayerSubsystems|GetEnhancedInputLocalPlayerSubsystem _asplayer_controller) "/Game/OSH/Input/IMC_Default_OSH.IMC_Default_OSH" 0 "(bIgnoreAllPressedKeysUntilRelease=True,bForceImmediately=False)"))

(event Collision|EventActorBeginOverlap
  (params (OtherActor :type Actor%20Object%20Reference)))

(event EventTick
  (params (DeltaSeconds :type Float%20%28single-precision%29))
  (bind _output_get (Variables|Default|SetCurrentFireCool (+ (Variables|Default|GetCurrentFireCool) DeltaSeconds)))
  (if (>= _output_get (Variables|Default|GetFireCool))
    (Variables|Default|SetCurrentFireCool (- (Variables|Default|GetCurrentFireCool) (Variables|Default|GetFireCool)))
    (Game|SpawnActorfromClass "/Game/OSH/Blueprint/BP_ProjectileBase.BP_ProjectileBase_C" (Transformation|GetWorldTransform (Variables|Default|GetArrow1)) "Undefined" 0 0)))

(fn ConstructionScript)